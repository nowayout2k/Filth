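; Player character Blueprint for a flipbook-sprite game, with four-direction movement, a timed attack and block grabbing.
; Axis input moves the character unless attacking, or, while grabbing a Block_BP found by the grab sphere, drives it via MoveBlock on a timeline.
; Player input is disabled through the game mode during the block move, then restored and the grab released.
; Each tick picks the idle, walk or attack flipbook from the last facing direction.
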(event `InputAxis|Up`
  (params (AxisValue :type "Float (single-precision)"))
  (bind _block (`self.Block`))
  (if (`self.isGrabbing`)
    (if (!= AxisValue 0.0)
      (bind _asfilth_game_mode_base_bp (cast `/Game/Blueprint/FilthGameModeBase_BP` (`GameplayStatics.GetGameMode`)))
      (`/Game/Blueprint/FilthGameModeBase_BP.SetPlayerInput` _asfilth_game_mode_base_bp false)
      (bind (_direction _scalealpha) (`Timeline|Timeline_1` :!via `PlayFromStart`)
        (:`Update`
          (`/Engine/EditorBlueprintResources/StandardMacros.IsValid` _block
            (:`Is Valid`
              (`/Game/Blueprint/Block_BP.MoveBlock` _block (`self.EMoveState`) _scalealpha))))
        (:`Finished`
          (bind _asfilth_game_mode_base_bp_2 (cast `/Game/Blueprint/FilthGameModeBase_BP` (`GameplayStatics.GetGameMode`)))
          (`/Game/Blueprint/FilthGameModeBase_BP.SetPlayerInput` _asfilth_game_mode_base_bp_2 true)
          (set `self.isGrabbing` false))))
    (elif (not (`self.GetIsAttacking`))
      (`self.AddMovementInput` (0.0 0.0 0.5) AxisValue))))

(event `InputAxis|Right`
  (params (AxisValue :type "Float (single-precision)"))
  (bind _block (`self.Block`))
  (if (`self.isGrabbing`)
    (if (!= AxisValue 0.0)
      (bind _asfilth_game_mode_base_bp (cast `/Game/Blueprint/FilthGameModeBase_BP` (`GameplayStatics.GetGameMode`)))
      (`/Game/Blueprint/FilthGameModeBase_BP.SetPlayerInput` _asfilth_game_mode_base_bp false)
      (bind (_direction _scalealpha) (`Timeline|Timeline_0` :!via `PlayFromStart`)
        (:`Update`
          (`/Engine/EditorBlueprintResources/StandardMacros.IsValid` _block
            (:`Is Valid`
              (`/Game/Blueprint/Block_BP.MoveBlock` _block (`self.EMoveState`) _scalealpha))))
        (:`Finished`
          (bind _asfilth_game_mode_base_bp_2 (cast `/Game/Blueprint/FilthGameModeBase_BP` (`GameplayStatics.GetGameMode`)))
          (`/Game/Blueprint/FilthGameModeBase_BP.SetPlayerInput` _asfilth_game_mode_base_bp_2 true)
          (set `self.isGrabbing` false))))
    (elif (not (`self.GetIsAttacking`))
      (`self.AddMovementInput` (0.5 0.0 0.0) AxisValue))))

(event `self.ReceiveTick`
  (params (DeltaSeconds :type "Float (single-precision)"))
  (`self.SetAnimationState`))

(event `InputAction|Attack`
  (params (Key :type "Key Structure"))
  (:`Pressed`
    (`self.SetIsAttacking` true)
    (`KismetSystemLibrary.Delay` 0.3333)
    (`self.SetIsAttacking` false)))

(event `InputAction|Grab`
  (params (Key :type "Key Structure"))
  (:`Pressed`
    (for _array_element (`PrimitiveComponent.GetOverlappingActors` (`self.GrabSphere`) "/Game/Blueprint/Block_BP.Block_BP_C")
      (bind _asblock_bp (cast `/Game/Blueprint/Block_BP` _array_element))
      (set `self.Block` _asblock_bp)
      (set `self.isGrabbing` true)))
  (:`Released`
    (set `self.isGrabbing` false)))

(fn `SetAnimationState`
  (if (`self.GetIsAttacking`)
    (`self.SetAttackAnimation`)
    (else
      (`self.SetLastMoveState`)
      (`self.SetMovementAnimation`))))

(fn `SetAttackAnimation`
  (`PaperFlipbookComponent.SetFlipbook` (`self.Sprite`) (select `/Game/Blueprint/EMoveState` (`self.EMoveState`) :`NewEnumerator0` "/Game/Animations/MaleChar/Attack/Male_Attack_UP.Male_Attack_UP" :`NewEnumerator1` "/Game/Animations/MaleChar/Attack/Male_Attack_Down.Male_Attack_Down" :`NewEnumerator2` "/Game/Animations/MaleChar/Attack/Male_Attack__Left.Male_Attack__Left" :`NewEnumerator3` "/Game/Animations/MaleChar/Attack/Male_Attack_Right.Male_Attack_Right" :!type "PaperFlipbook Object Reference")))

(fn `SetLastMoveState`
  (if (or (!= (`self.GetInputAxisValue`) 0.0) (!= (`self.GetInputAxisValue`) 0.0))
    (set `self.EMoveState` (select `bool` (> (`self.GetInputAxisValue`) 0.0) :`false` (select `bool` (< (`self.GetInputAxisValue`) 0.0) :`false` (select `bool` (> (`self.GetInputAxisValue`) 0.0) :`false` "NewEnumerator2" :`true` "NewEnumerator3" :!type "/Game/Blueprint/EMoveState Enum") :`true` "NewEnumerator1") :`true` "NewEnumerator0"))))

(fn `SetMovementAnimation`
  (bind _emovestate (`self.EMoveState`))
  (`PaperFlipbookComponent.SetFlipbook` (`self.Sprite`) (select `bool` (> (`KismetMathLibrary.VSize` (`self.GetVelocity`)) 0.0) :`false` (select `/Game/Blueprint/EMoveState` _emovestate :`NewEnumerator0` "/Game/Animations/MaleChar/Idle/Male_Idle_Up.Male_Idle_Up" :`NewEnumerator1` "/Game/Animations/MaleChar/Idle/Male_Idle_Down.Male_Idle_Down" :`NewEnumerator2` "/Game/Animations/MaleChar/Idle/Male_Idle_Left.Male_Idle_Left" :`NewEnumerator3` "/Game/Animations/MaleChar/Idle/Male_Idle_right.Male_Idle_right" :!type "PaperFlipbook Object Reference") :`true` (select `/Game/Blueprint/EMoveState` _emovestate :`NewEnumerator0` "/Game/Animations/MaleChar/Walk/Male_Walk_Up.Male_Walk_Up" :`NewEnumerator1` "/Game/Animations/MaleChar/Walk/Male_Walk_Down.Male_Walk_Down" :`NewEnumerator2` "/Game/Animations/MaleChar/Walk/Male_Walk_Left.Male_Walk_Left" :`NewEnumerator3` "/Game/Animations/MaleChar/Walk/Male_Walk_Right.Male_Walk_Right" :!type "PaperFlipbook Object Reference"))))

(fn `UserConstructionScript`)