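; FilthGameModeBase_BP is a game mode Blueprint that provides helper functions to freeze and resume play.
; SetPlayerInput enables or disables input on player character 0, zeroing its movement velocity when disabling so it stops immediately.
; SetGlobalTimeDilation switches global time dilation between normal speed when enabled and zero when disabled.
; Its event graph and construction script are empty, leaving these functions to be called from elsewhere.
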(fn `SetGlobalTimeDilation`
  (params (isEnabled :type Boolean))
  (if isEnabled
    (`GameplayStatics.SetGlobalTimeDilation` 1.0)
    (else
      (`GameplayStatics.SetGlobalTimeDilation` 0.0))))

(fn `SetPlayerInput`
  (params (isEnabled :type Boolean))
  (bind _returnvalue (`GameplayStatics.GetPlayerCharacter` 0))
  (if isEnabled
    (`self.EnableInput` (`GameplayStatics.GetPlayerCharacter` 0) (`GameplayStatics.GetPlayerController` 0))
    (else
      (`self.DisableInput` _returnvalue (`GameplayStatics.GetPlayerController` 0))
      (set `MovementComponent.Velocity` (0.0 0.0 0.0) (`Character.CharacterMovement` _returnvalue)))))

(fn `UserConstructionScript`)