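; Block_BP is a pushable block actor that slides a short fixed step up, down, left or right in the X-Z plane.
; TriggerPush calls SetPushVectors to store the current location and the offset target for the given direction, then plays a timeline from the start.
; Each timeline update calls MoveBlock, which lerps between those points with a swept move.
; The Push function is an empty stub.
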(event `TriggerPush`
  (params (Direction :type "/Game/Blueprint/EMoveState Enum" :default "NewEnumerator0"))
  (`self.SetPushVectors` Direction)
  (bind (_direction _alpha) (`Timeline|Timeline_0` :!via `PlayFromStart`)
    (:`Update`
      (`self.MoveBlock` (`self.Start Push Loc`) (`self.End Push Loc`) _alpha))))

(fn `MoveBlock`
  (params (`Start Push Loc` :type "Vector Structure") (`End Push Loc` :type "Vector Structure") (`Alpha value` :type "Float (double-precision)"))
  (`self.K2_SetActorLocation` (`KismetMathLibrary.VLerp` `Start Push Loc` `End Push Loc` `Alpha value`) true))

(fn `Push`
  (params (Direction :type "/Game/Blueprint/EMoveState Enum" :default "NewEnumerator0")))

(fn `SetPushVectors`
  (params (Direction :type "/Game/Blueprint/EMoveState Enum" :default "NewEnumerator0"))
  (set `self.Start Push Loc` (`self.K2_GetActorLocation`))
  (switch `/Game/Blueprint/EMoveState` Direction
    (:`NewEnumerator0`
      (set `self.End Push Loc` (+ (`self.K2_GetActorLocation`) (0.0 0.0 16.0))))
    (:`NewEnumerator1`
      (set `self.End Push Loc` (+ (`self.K2_GetActorLocation`) (0.0 0.0 -16.0))))
    (:`NewEnumerator2`
      (set `self.End Push Loc` (+ (`self.K2_GetActorLocation`) (-16.0 0.0 0.0))))
    (:`NewEnumerator3`
      (set `self.End Push Loc` (+ (`self.K2_GetActorLocation`) (16.0 0.0 0.0))))))

(fn `UserConstructionScript`)