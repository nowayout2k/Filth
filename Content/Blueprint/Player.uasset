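; Paper2D player mage that moves on the X-Z plane from the Up and Right input axes and plays four-direction animations.
; Each tick, SetAnimationState stores the last input direction, with vertical input taking priority over horizontal.
; It then sets the sprite's flipbook to the walk or idle animation for that direction, depending on whether velocity is non-zero.
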(event `InputAxis|Up`
  (params (AxisValue :type "Float (single-precision)"))
  (`self.AddMovementInput` (0.0 0.0 1.0) AxisValue))

(event `InputAxis|Right`
  (params (AxisValue :type "Float (single-precision)"))
  (`self.AddMovementInput` (1.0 0.0 0.0) AxisValue))

(event `self.ReceiveTick`
  (params (DeltaSeconds :type "Float (single-precision)"))
  (`self.SetAnimationState`))

(fn `SetAnimationState`
  (bind _last_move_state (`self.Last Move State`))
  (if (or (!= (`self.GetInputAxisValue`) 0.0) (!= (`self.GetInputAxisValue`) 0.0))
    (set `self.Last Move State` (select `bool` (> (`self.GetInputAxisValue`) 0.0) :`false` (select `bool` (< (`self.GetInputAxisValue`) 0.0) :`false` (select `bool` (> (`self.GetInputAxisValue`) 0.0) :`false` "NewEnumerator2" :`true` "NewEnumerator3" :!type "/Game/Blueprint/EMoveState Enum") :`true` "NewEnumerator1") :`true` "NewEnumerator0")))
  (`PaperFlipbookComponent.SetFlipbook` (`self.Sprite`) (select `bool` (> (`KismetMathLibrary.VSize` (`self.GetVelocity`)) 0.0) :`false` (select `/Game/Blueprint/EMoveState` _last_move_state :`NewEnumerator0` "/Game/Art/Mage/Animations/mage_IdleUp_Animation.mage_IdleUp_Animation" :`NewEnumerator1` "/Game/Art/Mage/Animations/mage_IdleDown_Animation.mage_IdleDown_Animation" :`NewEnumerator2` "/Game/Art/Mage/Animations/mage_IdleLeft_Aniamtion.mage_IdleLeft_Aniamtion" :`NewEnumerator3` "/Game/Art/Mage/Animations/mage_IdleRight_Animation.mage_IdleRight_Animation" :!type "PaperFlipbook Object Reference") :`true` (select `/Game/Blueprint/EMoveState` _last_move_state :`NewEnumerator0` "/Game/Art/Mage/Animations/mage_Up_Animation.mage_Up_Animation" :`NewEnumerator1` "/Game/Art/Mage/Animations/Mage_Down_Animation.Mage_Down_Animation" :`NewEnumerator2` "/Game/Art/Mage/Animations/mage_Left_Animation.mage_Left_Animation" :`NewEnumerator3` "/Game/Art/Mage/Animations/mage_Right_Animation.mage_Right_Animation" :!type "PaperFlipbook Object Reference"))))

(fn `UserConstructionScript`)