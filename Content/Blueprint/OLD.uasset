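; A player-controlled Paper2D character with four-directional walking, idling and attacking, moved by axis input along world X and Z.
; Pressing Attack sets a flag for about a third of a second, which blocks movement input and selects the attack animation.
; Each tick picks the sprite flipbook from that flag, velocity and the last input direction, with vertical input taking priority over horizontal.
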(event `InputAxis|Up`
  (params (AxisValue :type "Float (single-precision)"))
  (if (not (`self.IsAttacking`))
    (`self.AddMovementInput` (0.0 0.0 1.0) AxisValue)))

(event `InputAxis|Right`
  (params (AxisValue :type "Float (single-precision)"))
  (if (not (`self.IsAttacking`))
    (`self.AddMovementInput` (1.0 0.0 0.0) AxisValue)))

(event `self.ReceiveTick`
  (params (DeltaSeconds :type "Float (single-precision)"))
  (`self.SetAnimationState`))

(event `InputAction|Attack`
  (params (Key :type "Key Structure"))
  (:`Pressed`
    (set `self.IsAttacking` true)
    (`KismetSystemLibrary.Delay` 0.3333)
    (set `self.IsAttacking` false)))

(fn `SetAnimationState`
  (if (`self.IsAttacking`)
    (`self.SetAttackAnimation`)
    (else
      (`self.SetLastMoveState`)
      (`self.SetMovementAnimation`))))

(fn `SetAttackAnimation`
  (`PaperFlipbookComponent.SetFlipbook` (`self.Sprite`) (select `/Game/Blueprint/EMoveState` (`self.Last Move State`) :`NewEnumerator0` "/Game/Animations/MaleChar/Attack/Male_Attack_UP.Male_Attack_UP" :`NewEnumerator1` "/Game/Animations/MaleChar/Attack/Male_Attack_Down.Male_Attack_Down" :`NewEnumerator2` "/Game/Animations/MaleChar/Attack/Male_Attack__Left.Male_Attack__Left" :`NewEnumerator3` "/Game/Animations/MaleChar/Attack/Male_Attack_Right.Male_Attack_Right" :!type "PaperFlipbook Object Reference")))

(fn `SetLastMoveState`
  (if (or (!= (`self.GetInputAxisValue`) 0.0) (!= (`self.GetInputAxisValue`) 0.0))
    (set `self.Last Move State` (select `bool` (> (`self.GetInputAxisValue`) 0.0) :`false` (select `bool` (< (`self.GetInputAxisValue`) 0.0) :`false` (select `bool` (> (`self.GetInputAxisValue`) 0.0) :`false` "NewEnumerator2" :`true` "NewEnumerator3" :!type "/Game/Blueprint/EMoveState Enum") :`true` "NewEnumerator1") :`true` "NewEnumerator0"))))

(fn `SetMovementAnimation`
  (bind _last_move_state (`self.Last Move State`))
  (`PaperFlipbookComponent.SetFlipbook` (`self.Sprite`) (select `bool` (> (`KismetMathLibrary.VSize` (`self.GetVelocity`)) 0.0) :`false` (select `/Game/Blueprint/EMoveState` _last_move_state :`NewEnumerator0` "/Game/Animations/MaleChar/Idle/Male_Idle_Up.Male_Idle_Up" :`NewEnumerator1` "/Game/Animations/MaleChar/Idle/Male_Idle_Down.Male_Idle_Down" :`NewEnumerator2` "/Game/Animations/MaleChar/Idle/Male_Idle_Left.Male_Idle_Left" :`NewEnumerator3` "/Game/Animations/MaleChar/Idle/Male_Idle_right.Male_Idle_right" :!type "PaperFlipbook Object Reference") :`true` (select `/Game/Blueprint/EMoveState` _last_move_state :`NewEnumerator0` "/Game/Animations/MaleChar/Walk/Male_Walk_Up.Male_Walk_Up" :`NewEnumerator1` "/Game/Animations/MaleChar/Walk/Male_Walk_Down.Male_Walk_Down" :`NewEnumerator2` "/Game/Animations/MaleChar/Walk/Male_Walk_Left.Male_Walk_Left" :`NewEnumerator3` "/Game/Animations/MaleChar/Walk/Male_Walk_Right.Male_Walk_Right" :!type "PaperFlipbook Object Reference"))))

(fn `UserConstructionScript`)